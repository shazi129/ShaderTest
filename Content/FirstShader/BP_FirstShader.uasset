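; BP_FirstShader is a test Blueprint for drawing a selectable color into the RT_FirstShader render target through FirstShaderDrawRenderTarget.
; On BeginPlay it enables input from player controller 0, clears the target to gray and draws yellow.
; Keys 1, 2 and 3 print a debug message, switch the color to red, green or blue, and rerun the same draw call without clearing again.
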(event `self.ReceiveBeginPlay`
  (`self.EnableInput` (`GameplayStatics.GetPlayerController` 0))
  (`KismetRenderingLibrary.ClearRenderTarget2D` "/ShaderTest/FirstShader/RT_FirstShader.RT_FirstShader" (struct :`R` 0.5 :`G` 0.5 :`B` 0.5 :`A` 1.0))
  (set `self.Color` (struct :`R` 1.0 :`G` 1.0 :`A` 1.0))
  (`ShaderTestLibrary.FirstShaderDrawRenderTarget` null "/ShaderTest/FirstShader/RT_FirstShader.RT_FirstShader" (`self.Color`) :!label _label))

(event `Key|One`
  (params (Key :type "Key Structure"))
  (:`Pressed`
    (`KismetSystemLibrary.PrintString` "Press 1")
    (set `self.Color` (struct :`R` 1.0 :`A` 1.0))
    (goto _label)))

(event `Key|Two`
  (params (Key :type "Key Structure"))
  (:`Pressed`
    (`KismetSystemLibrary.PrintString` "Press 2")
    (set `self.Color` (struct :`G` 1.0 :`A` 1.0))
    (goto _label)))

(event `Key|Three`
  (params (Key :type "Key Structure"))
  (:`Pressed`
    (`KismetSystemLibrary.PrintString` "Press 3")
    (set `self.Color` (struct :`B` 1.0 :`A` 1.0))
    (goto _label)))

(fn `UserConstructionScript`)