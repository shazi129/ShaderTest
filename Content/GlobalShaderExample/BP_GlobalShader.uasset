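; BP_GlobalShader is an example actor that runs a UV displacement shader into the RT_GlobalShader render target.
; Each tick it clears the target to grey, then calls DrawUVDisplacementToRenderTarget with a FooCameraModel built from distortion coefficients K1 and K2.
; It enables input at BeginPlay, so W raises K1 and S raises K2 by a fixed increment, changing the displacement live.
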(event `self.ReceiveBeginPlay`
  (`self.EnableInput` (`GameplayStatics.GetPlayerController` 0)))

(event `self.ReceiveTick`
  (params (DeltaSeconds :type "Float (single-precision)"))
  (`KismetRenderingLibrary.ClearRenderTarget2D` "/ShaderTest/GlobalShaderExample/RT_GlobalShader.RT_GlobalShader" (struct :`R` 0.5 :`G` 0.5 :`B` 0.5 :`A` 1.0))
  (`LensDistortionBlueprintLibrary.DrawUVDisplacementToRenderTarget` (make `FooCameraModel` (`self.K1`) (`self.K2`)) 1.0 1.0 1.0 "/ShaderTest/GlobalShaderExample/RT_GlobalShader.RT_GlobalShader"))

(event `Key|W`
  (params (Key :type "Key Structure"))
  (:`Pressed`
    (set `self.K1` (+ (`self.K1`) (`self.inc`)))))

(event `Key|S`
  (params (Key :type "Key Structure"))
  (:`Pressed`
    (set `self.K2` (+ (`self.K2`) (`self.inc`)))))

(fn `UserConstructionScript`)