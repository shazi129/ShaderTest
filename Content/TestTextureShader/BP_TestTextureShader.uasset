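; Test actor that exercises a custom texture shader by drawing into the RT_TestTextureShader render target.
; On BeginPlay it clears the target to black and calls DrawTestTextureShaderRenderTarget with a struct holding three colors and a ColorIndex.
; Number keys 1 to 3 set ColorIndex and redraw the target to switch between the colors.
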(event `self.ReceiveBeginPlay`
  (`KismetRenderingLibrary.ClearRenderTarget2D` "/ShaderTest/TestTextureShader/RT_TestTextureShader.RT_TestTextureShader")
  (`ShaderTestLibrary.DrawTestTextureShaderRenderTarget` self "/ShaderTest/TestTextureShader/RT_TestTextureShader.RT_TestTextureShader" (make `TestTextureShaderStructData` (struct :`B` 1.0) (struct :`G` 1.0) (struct :`R` 1.0) (struct) (`self.ColorIndex`)) "/ShaderTest/TestTextureShader/298.298" :!label _label))

(event `Key|One`
  (params (Key :type "Key Structure"))
  (:`Pressed`
    (set `self.ColorIndex` 0)
    (goto _label)))

(event `Key|Two`
  (params (Key :type "Key Structure"))
  (:`Pressed`
    (set `self.ColorIndex` 1)
    (goto _label)))

(event `Key|Three`
  (params (Key :type "Key Structure"))
  (:`Pressed`
    (set `self.ColorIndex` 2)
    (goto _label)))

(fn `UserConstructionScript`)